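; Main menu player controller that shows the menu HUD and cursor and handles multiplayer session hosting, searching and joining through Advanced Sessions nodes.
; Hosting stores the server name as a session setting, then opens Lobby_Map as a listen server.
; Searching clears the menu's session box and fills it with one HUD_Session widget per result, with IsFindingSession set during the search and cleared only on success.
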(event `HUD Menu`
  ;[1 1 1] HUD Menu
  (bind _returnvalue (`|CreateWidget` "/Game/HUD/HUD_Menu.HUD_Menu_C"))
  (bind _output_get (set `self.HUD_Menu` _returnvalue))
  (`UserWidget.AddToViewport` _output_get 0))

(event `self.ReceiveBeginPlay`
  ;[1 1 1] Init
  (`self.HUD Menu`)
  (`self.Init Cursor`))

(event `Init Cursor`
  ;[1 1 1] Init Cursor
  (set `self.bShowMouseCursor` true)
  (`WidgetBlueprintLibrary.SetInputMode_GameAndUIEx` self null "LockInFullscreen" false))

(event `CreateSession`
  (params (`Session Name` :type String) (PublicConnections :type Integer))
  ;[1 1 1] Créer un serveur
  (`CreateSessionCallbackProxyAdvanced.CreateAdvancedSession` (`|MakeArray` (`AdvancedSessionsLibrary.MakeLiteralSessionPropertyString` "servername" `Session Name`)) self PublicConnections
    (:`OnSuccess`
      (`GameplayStatics.OpenLevel` "Lobby_Map" true "?listen"))))

(event `Rechercher`
  ;[1 1 1] Rechercher un serveur (clique sur le bouton rechercher au MAIN MENU)
  (`PanelWidget.ClearChildren` (`/Game/HUD/HUD_Menu.SessionBox` (`self.HUD_Menu`)))
  (set `self.IsFindingSession` true)
  (bind _results (`FindSessionsCallbackProxyAdvanced.FindSessionsAdvanced` self 99 false "AllServers")
    (:`OnSuccess`
      (for _array_element _results
        (bind _returnvalue (`|CreateWidget` "/Game/HUD/HUD_Session.HUD_Session_C" null _array_element))
        (`PanelWidget.AddChild` (`/Game/HUD/HUD_Menu.SessionBox` (`self.HUD_Menu`)) _returnvalue))
      (set `self.IsFindingSession` false))))

(event `JoinSession`
  (params (SearchResult :type "BlueprintSessionResult Structure (by ref)"))
  ;[1 1 1] Rejoindre un serveur par la recherche
  (`JoinSessionCallbackProxy.JoinSession` self SearchResult))

(fn `UserConstructionScript`)