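; PC_Player is a player Blueprint that sets up spatialized voice chat with push-to-talk.
; On BeginPlay it registers a remote talker and adds a VOIPTalker, then retries on a short delay until PlayerState is valid.
; It then registers the talker, drops the mic threshold and attaches voice attenuation to player controller 0's root component.
; The UseVoiceChat input toggles speaking through console commands, with debug prints.
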(event `self.ReceiveBeginPlay`
  (bind _playerstate (`self.PlayerState`))
  ;[1 0.1458 0.1458] Vocal Chat
  (bind _returnvalue (`AdvancedVoiceLibrary.RegisterRemoteTalker` (`AdvancedSessionsLibrary.GetUniqueNetID` null)))
  (`KismetSystemLibrary.PrintString` (`KismetStringLibrary.Concat_StrStr` "SetVocal:" (`KismetStringLibrary.Conv_BoolToString` _returnvalue)) true true (struct :`G` 0.66 :`B` 1.0 :`A` 1.0) 10.0)
  (bind _returnvalue_2 (`AddComponent|NODE_AddVOIPTalker-2`))
  (bind _output_get (set `self.VOIP` _returnvalue_2))
  (`/Engine/EditorBlueprintResources/StandardMacros.IsValid` _playerstate :!label _label
    (:`Is Valid`
      (`VOIPTalker.RegisterWithPlayerState` _output_get _playerstate)
      (`VOIPStatics.SetMicThreshold` -9999999.0)
      (set `VOIPTalker.Settings` (make `VoiceSettings` (`Actor.RootComponent` (`GameplayStatics.GetPlayerController` 0)) "/Game/Audio/SoundAttenuartion.SoundAttenuartion") (`self.VOIP`)))
    (:`Is Not Valid`
      (`KismetSystemLibrary.Delay` 0.2)
      (goto _label))))

(event `InputAction|UseVoiceChat`
  (params (Key :type "Key Structure"))
  ;[1 0.1458 0.1458] Vocal Chat
  ;;[1 1 1] Push to Talk
  (:`Pressed`
    (`KismetSystemLibrary.ExecuteConsoleCommand` "ToggleSpeaking 1" null)
    (`KismetSystemLibrary.PrintString` "Press"))
  (:`Released`
    (`KismetSystemLibrary.ExecuteConsoleCommand` "ToggleSpeaking 0" null)
    (`KismetSystemLibrary.PrintString` "Relache")))

(fn `UserConstructionScript`)