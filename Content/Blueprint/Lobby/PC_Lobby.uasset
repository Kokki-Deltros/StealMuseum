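; Lobby player controller that sets up the lobby screen and handles player list updates, kicks and bans.
; On BeginPlay it shows the cursor, switches to Game and UI input, and creates the HUD_Lobby widget.
; Events forward add and clear requests to that widget's player list.
; Kick opens Menu_Map with the listen option and destroys the session, while ban calls BanPlayer with an empty reason.
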(event `self.ReceiveBeginPlay`
  (set `self.bShowMouseCursor` true)
  (`WidgetBlueprintLibrary.SetInputMode_GameAndUIEx` self null "LockInFullscreen" false)
  (`self.HUD Lobby`))

(event `HUD Lobby`
  (bind _returnvalue (`|CreateWidget` "/Game/HUD/HUD_Lobby.HUD_Lobby_C"))
  (bind _output_get (set `self.HUD_Lobby` _returnvalue))
  (`UserWidget.AddToViewport` _output_get 0))

(event `ClearPlayerList`
  ;[1 1 1] Clear player list in lobby
  (`/Game/HUD/HUD_Lobby.ClearPlayerList` (`self.HUD_Lobby`)))

(event `KickPlayer`
  ;[1 1 1] Kick player of server
  (`GameplayStatics.OpenLevel` "Menu_Map" true "?listen")
  (`DestroySessionCallbackProxy.DestroySession` self))

(event `AddPlayer`
  (params (Player :type Text) (PlayerIndex :type Integer))
  ;[1 1 1] Add player in player list in lobby
  (`/Game/HUD/HUD_Lobby.AddPlayerToList` (`self.HUD_Lobby`) Player PlayerIndex))

(event `BanPlayer`
  ;[1 1 1] Ban player of server
  (`AdvancedSessionsLibrary.BanPlayer` null))

(fn `UserConstructionScript`)