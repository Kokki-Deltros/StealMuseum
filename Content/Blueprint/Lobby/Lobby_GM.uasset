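; Lobby game mode that tracks connected PC_Lobby controllers and keeps the lobby's player count and name lists current.
; Logins, after a half-second delay, and logouts pass the controller count to Lobby_GS, then call UpdateServer.
; UpdateServer clears and rebuilds every controller's player list with names and array indices.
; KickPlayer uses that index to tell the matching controller to kick itself.
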(event `self.K2_PostLogin`
  (params (NewPlayer :type "PlayerController Object Reference"))
  (bind _aspc_lobby (cast `/Game/Blueprint/Lobby/PC_Lobby` NewPlayer))
  (`KismetArrayLibrary.Array_Add` (`self.AllPC`) _aspc_lobby)
  (`KismetSystemLibrary.Delay` 0.5)
  (bind _aslobby_gs (cast `/Game/Blueprint/Lobby/Lobby_GS` (`GameplayStatics.GetGameState`)))
  (`/Game/Blueprint/Lobby/Lobby_GS.Update Players` _aslobby_gs (`KismetArrayLibrary.Array_Length` (`self.AllPC`)))
  (`self.UpdateServer`))

(event `self.K2_OnLogout`
  (params (ExitingController :type "Controller Object Reference"))
  (bind _aspc_lobby (cast `/Game/Blueprint/Lobby/PC_Lobby` ExitingController))
  (`KismetArrayLibrary.Array_RemoveItem` (`self.AllPC`) _aspc_lobby)
  (bind _aslobby_gs (cast `/Game/Blueprint/Lobby/Lobby_GS` (`GameplayStatics.GetGameState`)))
  (`/Game/Blueprint/Lobby/Lobby_GS.Update Players` _aslobby_gs (`KismetArrayLibrary.Array_Length` (`self.AllPC`)))
  (`self.UpdateServer`))

(event `UpdateServer`
  (for _array_element (`self.AllPC`)
    (`/Game/Blueprint/Lobby/PC_Lobby.ClearPlayerList` _array_element)
    (for (_array_element_2 _array_index) (`self.AllPC`)
      (`/Game/Blueprint/Lobby/PC_Lobby.AddPlayer` _array_element (`KismetTextLibrary.Conv_StringToText` (`AdvancedSessionsLibrary.GetPlayerName` _array_element_2)) _array_index))))

(event `KickPlayer`
  (params (`Player index` :type Integer))
  (`/Game/Blueprint/Lobby/PC_Lobby.KickPlayer` (`|GetArrayItem` (`self.AllPC`) `Player index`)))

(fn `UserConstructionScript`)